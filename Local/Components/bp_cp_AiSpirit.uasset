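; AI spirit component that binds an AI controller to the NPC body it controls and links to a mind actor.
; Each server tick, it hands the controller to the pawn's HumanTalamus component if that lacks AI, then records the pawn as its body.
; Protocol offers store the mind actor and reply with acceptance, while closing statements are forwarded to it.
; The testing, key-settings and stack-status protocol functions are empty stubs.
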(event `self.ReceiveTick`
  (params (DeltaSeconds :type "Float (single-precision)"))
  (bind _mycontroller (`self.MyController`))
  (if (`KismetSystemLibrary.IsServer`)
    (`/Engine/EditorBlueprintResources/StandardMacros.IsValid` _mycontroller
      (:`Is Valid`
        (bind _asbase_npc (cast `/Game/Characters/BaseNPC` (`Controller.K2_GetPawn` _mycontroller)))
        (bind _returnvalue (`Actor.GetComponentByClass` _asbase_npc "/Game/Mods/tradeboxmod/Components/bp_cp_HumanTalamus.bp_cp_HumanTalamus_C"))
        (if (not (`/Game/Mods/tradeboxmod/Components/bp_cp_HumanTalamus.GetHasAI` _returnvalue))
          (`/Game/Mods/tradeboxmod/Components/bp_cp_HumanTalamus.SVR_ReceiveAI` _returnvalue _mycontroller)
          (set `self.MyBody` _asbase_npc))))))

(event `/Game/ModsShared/tradeboxmod/bp_if_Protocol.ProtocolClosed`
  (params (ClosingStatement :type String))
  (message `/Game/ModsShared/tradeboxmod/bp_if_Protocol.ProtocolClosed` (`self.MindActor`) ClosingStatement)
  (`KismetSystemLibrary.PrintString` ClosingStatement false false (struct :`G` 0.059178 :`B` 1.0 :`A` 1.0) 10.0))

(event `/Game/ModsShared/tradeboxmod/bp_if_Protocol.ProtocolOffer`
  (params (MindActor :type "ActorComponent Object Reference"))
  (bind _output_get (set `self.MindActor` MindActor))
  (message `/Game/ModsShared/tradeboxmod/bp_if_Protocol.ProtocolAcceptAiSpirit` _output_get self))

(fn `ProtocolFNeedsTesting`
  (returns (DoTest :type Boolean))
  (return false))

(fn `ProtocolGetKeySettings`
  (returns (MainModKey :type "Key Structure") (ReceptiveModKey :type "Key Structure"))
  (return))

(fn `ProtocolStackStatus`
  (returns (SerialBool :type String))
  (return ""))