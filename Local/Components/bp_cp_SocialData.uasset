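; Conan Exiles character component that holds a player's or NPC's social data: known concepts, personality and mod key settings.
; Concepts live in an array indexed by a name map, serialized on update for storage.
; Personality is a shuffled Arcanum order cached as a string, loaded when the mind protocol with the HumanTalamus component closes.
; Server-bound damage events apply Nergal item effects, refilling owner health or lowering victims' health and consciousness.
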(event `MakeConceptSerial`
  (bind _knowledgebase (`self.KnowledgeBase`))
  (`KismetSystemLibrary.PrintString` (`KismetStringLibrary.Concat_StrStr` "Serializing memory:" (`KismetStringLibrary.Conv_IntToString` (`KismetArrayLibrary.Array_Length` _knowledgebase))) false false (struct :`G` 0.130607 :`B` 1.0 :`A` 1.0) 5.0)
  (for _array_element _knowledgebase
    (`KismetArrayLibrary.Array_AddUnique` (`self.KnownConcepts`) (`/Game/ModsShared/tradeboxmod/bp_lib_Serialization.SerializeConcept` _array_element))))

(event `MakeConceptArray`
  (bind _knownconcepts (`self.KnownConcepts`))
  (bind _knowledgebase (`self.KnowledgeBase`))
  (`KismetSystemLibrary.PrintString` (`KismetStringLibrary.Concat_StrStr` "Start memory:" (`KismetStringLibrary.Conv_IntToString` (`KismetArrayLibrary.Array_Length` _knownconcepts))) false false (struct :`G` 0.130607 :`B` 1.0 :`A` 1.0) 5.0)
  (for _array_element _knownconcepts
    (`KismetArrayLibrary.Array_AddUnique` _knowledgebase (`/Game/ModsShared/tradeboxmod/bp_lib_Serialization.DeserializeConcept` _array_element)))
  (for (_array_element_2 _array_index) _knowledgebase
    (`BlueprintMapLibrary.Map_Add` (`self.ConceptMap`) (`.Concept_12_02C6FF2F4715DFD465EAD8A7758E2927` (break `/Game/ModsShared/tradeboxmod/DataStructures/tbs_KnownConcepts` _array_element_2)) _array_index)))

(event `self.ReceiveBeginPlay`
  (bind _asconan_character (cast `ConanCharacter` (`self.GetOwner`)))
  (if (`ConanCharacter.IsABrush` _asconan_character)
    _
    (elif (`KismetSystemLibrary.IsServer`)
      (`self.SVR_FindingMind`)
      (add `Actor.OnTakeAnyDamage` _asconan_character (delegate `TakenDamage`))
      (add `ConanCharacter.SignalOnDamageDelivered` _asconan_character (delegate `SignalOnDamageDelivered_Event_0`)))))

(event `TakenDamage`
  (params (DamagedActor :type "Actor Object Reference") (Damage :type "Float (double-precision)") (DamageType :type "DamageType Object Reference") (InstigatedBy :type "Controller Object Reference") (DamageCauser :type "Actor Object Reference") (DamageEventID :type Integer))
  (`self.ManagerTakenDamage` DamagedActor Damage DamageType InstigatedBy DamageCauser DamageEventID))

(event `SignalOnDamageDelivered_Event_0`
  (params (Attacker :type "ConanCharacter Object Reference") (Target :type "ConanCharacter Object Reference") (Killed :type Boolean))
  (`self.ManagerDamageDelivered` Attacker Target Killed))

(event `SVR_LoadPersonality`
  (bind _returnvalue (enumcount `/Game/Mods/tradeboxmod/SystemTables/enum_Arcana`))
  (bind _arcanumorder (`self.ArcanumOrder`))
  (bind _arcanumstring (`self.ArcanumString`))
  (bind _returnvalue_2 (`KismetArrayLibrary.Array_Length` _arcanumorder))
  (bind (_asbase_player_char _bsuccess) (cast `/Game/Characters/BasePlayerChar` (`self.GetOwner`) :!pure true))
  (bind _returnvalue_3 (< _returnvalue_2 _returnvalue))
  (`KismetSystemLibrary.PrintString` (select `bool` _bsuccess :`false` "NPC Social" :`true` "Player Social") false false (select `bool` _bsuccess :`false` (struct :`R` 0.905 :`B` 0.606036 :`A` 1.0) :`true` (struct :`G` 0.485 :`B` 0.116375 :`A` 1.0) :!type "LinearColor Structure") 20.0)
  (`|ExecutionSequence`
    (:`then_0`
      (`KismetSystemLibrary.PrintString` (`KismetStringLibrary.Concat_StrStr` "Cards:" (`KismetStringLibrary.Conv_IntToString` _returnvalue_2) "/" (`KismetStringLibrary.Conv_IntToString` _returnvalue) ":" (`KismetStringLibrary.Conv_BoolToString` _returnvalue_3)) false false (struct :`G` 0.66 :`B` 1.0 :`A` 1.0) 20.0)
      (`KismetSystemLibrary.PrintString` _arcanumstring false false (struct :`R` 0.545 :`G` 0.170663 :`A` 1.0) 20.0 :!label _label))
    (:`then_1`
      (if _returnvalue_3
        (for _index (range _returnvalue)
          (`KismetArrayLibrary.Array_Set` _arcanumorder _index (`KismetMathLibrary.Conv_IntToByte` _index) true))
        (`KismetArrayLibrary.Array_Shuffle` _arcanumorder)))
    (:`then_2`
      (if (<= (`KismetStringLibrary.Len` (`self.ArcanumString`)) 2)
        (set `self.ArcanumString` "")
        (for _array_element _arcanumorder
          (set `self.ArcanumString` (`KismetStringLibrary.Concat_StrStr` _arcanumstring (`KismetStringLibrary.Trim` (`KismetStringLibrary.Conv_ByteToString` _array_element)) ".")))
        (goto _label)))
    (:`then_3`
      (`KismetSystemLibrary.PrintString` (`self.ArcanumString`) false false (struct :`R` 1.0 :`G` 0.837406 :`A` 1.0) 20.0))))

(event `/Game/ModsShared/tradeboxmod/bp_if_Protocol.ProtocolClosed`
  (params (ClosingStatement :type String))
  (message `/Game/ModsShared/tradeboxmod/bp_if_Protocol.ProtocolClosed` (`self.MindActor`) ClosingStatement)
  (`self.SVR_LoadPersonality`))

(event `/Game/ModsShared/tradeboxmod/bp_if_Protocol.ProtocolOffer`
  (params (MindActor :type "ActorComponent Object Reference"))
  (bind _output_get (set `self.MindActor` MindActor))
  (message `/Game/ModsShared/tradeboxmod/bp_if_Protocol.ProtocolAcceptSocialData` _output_get self))

(event `/Game/ModsShared/tradeboxmod/bp_if_Protocol.ProtocolSetMainKey`
  (params (SelectedKey :type "Key Structure" :default "AnyKey"))
  (set `self.ModSettingsKey` SelectedKey))

(event `/Game/ModsShared/tradeboxmod/bp_if_Protocol.ProtocolSetReceptiveKey`
  (params (SelectedKey :type "Key Structure" :default "AnyKey"))
  (set `self.ModReceptiveKey` SelectedKey))

(event `SVR_FindingMind`
  (bind _asconan_character (cast `ConanCharacter` (`self.GetOwner`)))
  (if (not (`ConanCharacter.IsABrush` _asconan_character))
    (`/Engine/EditorBlueprintResources/StandardMacros.IsValid` (`self.MindActor`)
      (:`Is Valid`
        (bind _returnvalue (`Actor.GetComponentByClass` _asconan_character "/Game/Mods/tradeboxmod/Components/bp_cp_HumanTalamus.bp_cp_HumanTalamus_C"))
        (`/Game/Mods/tradeboxmod/Components/bp_cp_HumanTalamus.SVR_ReceiveBody` _returnvalue _asconan_character)
        (set `self.MindActor` _returnvalue)))))

(event `UpdateConcept`
  (params (Concept :type "String (by ref)") (Score :type "Float (double-precision)") (Feelings :type "Float (double-precision)") (Stage :type "Float (double-precision)") (Control :type Integer))
  (bind _returnvalue (`KismetStringLibrary.Conv_StringToName` Concept))
  (bind _knowledgebase (`self.KnowledgeBase`))
  (bind (_value _returnvalue_2) (`BlueprintMapLibrary.Map_Find` (`self.ConceptMap`) _returnvalue))
  (bind _tbs_knownconcepts (make `/Game/ModsShared/tradeboxmod/DataStructures/tbs_KnownConcepts` _returnvalue Score Feelings Stage Control))
  (if _returnvalue_2
    (`KismetArrayLibrary.Array_Set` _knowledgebase _value _tbs_knownconcepts true)
    (else
      (bind _returnvalue_3 (`KismetArrayLibrary.Array_AddUnique` _knowledgebase _tbs_knownconcepts))
      (`BlueprintMapLibrary.Map_Add` (`self.ConceptMap`) _returnvalue _returnvalue_3)))
  (`self.MakeConceptSerial`))

(event `ManagerTakenDamage`
  (params (DamagedActor :type "Actor Object Reference") (Damage :type "Float (double-precision)") (DamageType :type "DamageType Object Reference") (InstigatedBy :type "Controller Object Reference") (DamageCauser :type "Actor Object Reference") (DamageEventID :type Integer))
  (bind _asconan_character (cast `ConanCharacter` DamagedActor :!pure true))
  (bind (_handprint _ringsouls) (`self.HasNergalItems` (`Controller.K2_GetPawn` InstigatedBy)))
  (bind _asconan_character_2 (cast `ConanCharacter` (`self.GetOwner`) :!pure true))
  (`|ExecutionSequence`
    (:`then_0`
      (if (`self.HasNergalItems` null)
        (`ConanCharacter.SetIntStat` _asconan_character_2 "HealthCurrent" (`ConanCharacter.GetIntStat` _asconan_character_2 "HealthMax" "Full"))))
    (:`then_1`
      (if (not (or (`.bSuccess` (cast `/Game/Characters/BasePlayerChar` DamagedActor :!pure true)) (`.bSuccess` (cast `/Game/Characters/NPCs/Humanoid/PersistentHumanoidNPC` DamagedActor :!pure true))))
        (`|ExecutionSequence`
          (:`then_0`
            (if _ringsouls
              (`ConanCharacter.SetIntStat` _asconan_character "ConsciousnessCurrent" 1)))
          (:`then_1`
            (if _handprint
              (`ConanCharacter.SetIntStat` _asconan_character "HealthCurrent" 5))))))))

(event `ManagerDamageDelivered`
  (params (Attacker :type "ConanCharacter Object Reference") (Target :type "ConanCharacter Object Reference") (Killed :type Boolean)))

(fn `GetConceptScore`
  (params (Concept :type "String (by ref)"))
  (returns (Found :type Boolean) (Score :type "Float (double-precision)") (Feelings :type "Float (double-precision)") (Stage :type "Float (double-precision)") (Control :type Integer))
  (bind (_value _returnvalue) (`BlueprintMapLibrary.Map_Find` (`self.ConceptMap`) (`KismetStringLibrary.Conv_StringToName` Concept)))
  (bind (_concept _score _feelings _stage _control) (break `/Game/ModsShared/tradeboxmod/DataStructures/tbs_KnownConcepts` (`KismetArrayLibrary.Array_Get` (`self.KnowledgeBase`) _value)))
  (if _returnvalue
    (return true _score _feelings _stage _control)
    (else
      (return false 0.0 0.0 0.0 0))))

(fn `HasNergalItems`
  (params (Character :type "Actor Object Reference"))
  (returns (HandPrint :type Boolean) (RingSouls :type Boolean))
  (locals (ItemsHave :type "Array of Boolean"))
  (bind _itemshave (`local.ItemsHave`))
  (for (_array_element _array_index) (`|MakeArray` 190701 190702)
    (`KismetArrayLibrary.Array_Set` _itemshave _array_index (> (`ItemInventory.GetNumberOfItemsByTemplate` (`ItemInventory.GetInventoryByType` (select `bool` (`KismetSystemLibrary.IsValid` Character) :`false` (`self.GetOwner`) :`true` Character) "Backpack") _array_element) 0) true))
  (return (`KismetArrayLibrary.Array_Get` _itemshave) (`KismetArrayLibrary.Array_Get` _itemshave 1)))

(fn `MakeTaskMap`
  (returns (TaskMap1 :type "Map of Float (double-precision) to Integer"))
  (locals (TaskMap :type "Map of Float (double-precision) to Integer"))
  (bind _taskmap (`local.TaskMap`))
  (for (_array_element _array_index) (`self.TaskStarting`)
    (`BlueprintMapLibrary.Map_Add` _taskmap _array_element (`KismetArrayLibrary.Array_Get` (`self.TaskRecipes`) _array_index)))
  (return _taskmap))

(fn `ProtocolFNeedsTesting`
  (returns (DoTest :type Boolean))
  (return false))

(fn `ProtocolGetKeySettings`
  (returns (MainModKey :type "Key Structure") (ReceptiveModKey :type "Key Structure"))
  (return (`self.ModSettingsKey`) (`self.ModReceptiveKey`)))

(fn `ProtocolStackStatus`
  (returns (SerialBool :type String))
  (return ""))