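; Blueprint function library of stateless math helpers for vectors, transforms and phase-based row redirects.
; Min/max helpers feed midpoint functions, while per-axis scale and translate helpers feed ProcessChange, which edits transforms from custom data.
; Phasing functions scan float redirect arrays by threshold, exact or absolute match; the last match replaces the original row.
; Also includes integer summing, X-location mirroring, proximity and facing checks, and a hard-coded body-part index list.
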(fn `ArraySumInteger`
  (params (Array :type "Array of Integer"))
  (returns (Sum :type Integer))
  (locals (Total :type Integer))
  (bind _total (`local.Total`))
  (set `local.Total` 0)
  (for _array_element Array
    (set `local.Total` (+ _total _array_element)))
  (return _total))

(fn `BodypartArray`
  (returns (Array :type "Array of String"))
  (return (`|MakeArray` "2,3,8" "0,1,7" "5,6,11,12")))

(fn `FloatMiddle`
  (params (FloatA :type "Float (double-precision)") (FloatB :type "Float (double-precision)"))
  (returns (Middle :type "Float (double-precision)"))
  (bind (_floatmin _floatmax) (`self.FloatMinMax` FloatA FloatB))
  (return (- _floatmax (/ (- _floatmax _floatmin) 2.0))))

(fn `FloatMinMax`
  (params (FloatA :type "Float (double-precision)") (FloatB :type "Float (double-precision)"))
  (returns (FloatMin :type "Float (double-precision)") (FloatMax :type "Float (double-precision)"))
  (return (`KismetMathLibrary.FMin` FloatA FloatB) (`KismetMathLibrary.FMax` FloatA FloatB)))

(fn `GetLocationDirections`
  (params (WhereYouAre :type "Vector Structure (by ref)") (YourRotation :type "Rotator Structure") (WhereYouGoing :type "Vector Structure (by ref)") (AskedRotation :type "Rotator Structure") (HastaRadius :type "Float (double-precision)"))
  (returns (Closeby :type Boolean) (Facing :type Boolean) (Rotated :type Boolean) (Distance :type "Float (double-precision)") (ToLookAt :type "Rotator Structure") (HeightDelta :type "Float (double-precision)") (HastaRadiumRp :type "Float (double-precision)"))
  (bind _returnvalue (- WhereYouAre WhereYouGoing))
  (bind _returnvalue_2 (`KismetMathLibrary.GetForwardVector` YourRotation))
  (bind _returnvalue_3 (`KismetMathLibrary.VSize` _returnvalue))
  (return (<= _returnvalue_3 HastaRadius) (< (`KismetMathLibrary.DegAcos` (`KismetMathLibrary.Dot_VectorVector` (`KismetMathLibrary.Normal` _returnvalue) _returnvalue_2)) 10.0) (< (`KismetMathLibrary.DegAcos` (`KismetMathLibrary.Dot_VectorVector` _returnvalue_2 (`KismetMathLibrary.GetForwardVector` AskedRotation))) 10.0) _returnvalue_3 (`KismetMathLibrary.FindLookAtRotation` WhereYouAre WhereYouGoing) (- (.z WhereYouGoing) (.z WhereYouAre)) HastaRadius))

(fn `MiddleGroundVector`
  (params (VectorMax :type "Vector Structure") (VectorMin :type "Vector Structure"))
  (returns (VectorNormal :type "Vector Structure"))
  (return (`KismetMathLibrary.MakeVector` (`self.FloatMiddle` (.x VectorMax) (.x VectorMin)) (`self.FloatMiddle` (.y VectorMax) (.y VectorMin)) (`self.FloatMiddle` (.z VectorMax) (.z VectorMin)))))

(fn `MiddlePlaneVector`
  (params (VectorMax :type "Vector Structure") (VectorMin :type "Vector Structure") (Normal :type "Vector Structure"))
  (returns (MiddleVectorNormal :type "Vector Structure"))
  (return (`self.NormalizeZ` (`self.MiddleGroundVector` VectorMax VectorMin) Normal)))

(fn `MirrorTransform`
  (params (InTransform :type "Transform Structure (by ref)"))
  (returns (ReturnTransform :type "Transform Structure"))
  (return (`KismetMathLibrary.MakeTransform` (`KismetMathLibrary.MakeVector` (* (.x (.location InTransform)) -1.0) (.y (.location InTransform)) (.z (.location InTransform))) (.rotation InTransform) (.scale InTransform))))

(fn `NormalizeZ`
  (params (Vector :type "Vector Structure") (Normal :type "Vector Structure"))
  (returns (VectorNormal :type "Vector Structure"))
  (return (`KismetMathLibrary.MakeVector` (.x Vector) (.y Vector) (.z Normal))))

(fn `ProcessAbsoluteFloatPhasing`
  (params (FloatPhasingArray :type "/Game/ModsShared/tradeboxmod/DataStructures/tbs_FloatBasedRedirect Structure") (PhaseIsIn :type "Float (double-precision)") (OriginalRow :type Name))
  (returns (ProcessedRow :type Name))
  (locals (LastPhaseChecked :type "Float (double-precision)") (ProcessRow :type Name) (LastCheck :type "Float (double-precision)"))
  (set `local.ProcessRow` OriginalRow)
  (set `local.LastPhaseChecked` 0.0)
  (for _array_element (`.FloatRedirects_4_B0D2B2B84AF2640805164783FA6DB125` (break `/Game/ModsShared/tradeboxmod/DataStructures/tbs_FloatBasedRedirect` FloatPhasingArray))
    (bind (_phasingflotstat _redirectrow) (break `/Game/ModsShared/tradeboxmod/DataStructures/dat_FloatPhasingPairs` _array_element))
    (if (`.AbsoluteCondition` (`self.ProcessFloatPhasing` PhaseIsIn _phasingflotstat))
      (set `local.ProcessRow` _redirectrow)))
  (return (`local.ProcessRow`)))

(fn `ProcessChange`
  (params (InTransform :type "Transform Structure (by ref)") (CustomData :type "/Game/ModsShared/tradeboxmod/DataStructures/dat_CustomizationCmd Structure (by ref)"))
  (returns (ReturnValue :type "Transform Structure"))
  (bind (_command _index _x _y _z _offset _l _w _h _scale) (break `/Game/ModsShared/tradeboxmod/DataStructures/dat_CustomizationCmd` CustomData))
  (return (`KismetMathLibrary.MakeTransform` (`self.TranslateVectors` (.location InTransform) _offset _x _y _z) (.rotation InTransform) (`self.ScaleVectors` (.scale InTransform) _scale _l _w _h))))

(fn `ProcessExactFloatPhasing`
  (params (FloatPhasingArray :type "/Game/ModsShared/tradeboxmod/DataStructures/tbs_FloatBasedRedirect Structure") (PhaseIsIn :type "Float (double-precision)") (Original :type Name))
  (returns (ProcessedRow :type Name))
  (locals (LastPhaseChecked :type "Float (double-precision)") (ProcessRow :type Name) (LastCheck :type "Float (double-precision)"))
  (set `local.ProcessRow` Original)
  (set `local.LastPhaseChecked` 0.0)
  (for _array_element (`.FloatRedirects_4_B0D2B2B84AF2640805164783FA6DB125` (break `/Game/ModsShared/tradeboxmod/DataStructures/tbs_FloatBasedRedirect` FloatPhasingArray))
    (bind (_phasingflotstat _redirectrow) (break `/Game/ModsShared/tradeboxmod/DataStructures/dat_FloatPhasingPairs` _array_element))
    (if (`.ConditionPhase` (`self.ProcessFloatPhasing` PhaseIsIn _phasingflotstat))
      (set `local.ProcessRow` _redirectrow)))
  (return (`local.ProcessRow`)))

(fn `ProcessFloatPhasing`
  (params (PhaseIsIn :type "Float (double-precision)") (PhaseSought :type "Float (double-precision)") (LastPhaseChecked :type "Float (double-precision)"))
  (returns (IsSought :type Boolean) (HasPhased :type Boolean) (HasPhasedOverall :type Boolean) (ConditionPhase :type Boolean) (AbsoluteCondition :type Boolean) (PhaseOverall :type "Float (double-precision)"))
  (bind _returnvalue (>= PhaseIsIn LastPhaseChecked))
  (bind _returnvalue_2 (`KismetMathLibrary.Abs` PhaseSought))
  (bind _returnvalue_3 (>= PhaseIsIn _returnvalue_2))
  (return (< PhaseSought 0.0) _returnvalue_3 (and _returnvalue_3 _returnvalue) (== PhaseIsIn PhaseSought) (== PhaseIsIn _returnvalue_2) (select `bool` _returnvalue :`false` LastPhaseChecked :`true` PhaseIsIn)))

(fn `ProcessOverallFloatPhasing`
  (params (FloatPhasingArray :type "/Game/ModsShared/tradeboxmod/DataStructures/tbs_FloatBasedRedirect Structure") (PhaseIsIn :type "Float (double-precision)") (OriginalRow :type Name))
  (returns (ProcessedRow :type Name))
  (locals (LastPhaseChecked :type "Float (double-precision)") (ProcessRow :type Name) (LastCheck :type "Float (double-precision)"))
  (set `local.ProcessRow` OriginalRow)
  (set `local.LastPhaseChecked` 0.0)
  (for _array_element (`.FloatRedirects_4_B0D2B2B84AF2640805164783FA6DB125` (break `/Game/ModsShared/tradeboxmod/DataStructures/tbs_FloatBasedRedirect` FloatPhasingArray))
    (bind (_phasingflotstat _redirectrow) (break `/Game/ModsShared/tradeboxmod/DataStructures/dat_FloatPhasingPairs` _array_element))
    (bind (_issought _hasphased _hasphasedoverall _conditionphase _absolutecondition _phaseoverall) (`self.ProcessFloatPhasing` PhaseIsIn _phasingflotstat (`local.LastPhaseChecked`)))
    (if _hasphasedoverall
      (set `local.ProcessRow` _redirectrow)
      (set `local.LastCheck` _phaseoverall)))
  (return (`local.ProcessRow`)))

(fn `ScaleVectors`
  (params (OriginalVector :type "Vector Structure") (Factor :type "Float (double-precision)") (GrowX :type Boolean) (GrowY :type Boolean) (GrowZ :type Boolean))
  (returns (ScaledVector :type "Vector Structure"))
  (bind _x (.x OriginalVector))
  (bind _y (.y OriginalVector))
  (bind _z (.z OriginalVector))
  (return (`KismetMathLibrary.MakeVector` (select `bool` GrowX :`false` _x :`true` (* _x Factor)) (select `bool` GrowY :`false` _y :`true` (* _y Factor)) (select `bool` GrowZ :`false` _z :`true` (* _z Factor)))))

(fn `TranslateVectors`
  (params (OriginalVector :type "Vector Structure") (Factor :type "Float (double-precision)") (GrowX :type Boolean) (GrowY :type Boolean) (GrowZ :type Boolean))
  (returns (ScaledVector :type "Vector Structure"))
  (bind _x (.x OriginalVector))
  (bind _y (.y OriginalVector))
  (bind _z (.z OriginalVector))
  (return (`KismetMathLibrary.MakeVector` (select `bool` GrowX :`false` _x :`true` (+ _x Factor)) (select `bool` GrowY :`false` _y :`true` (+ _y Factor)) (select `bool` GrowZ :`false` _z :`true` (+ _z Factor)))))

(fn `VectorMinMax`
  (params (VectorA :type "Vector Structure") (VectorB :type "Vector Structure"))
  (returns (VectornMin :type "Vector Structure") (VectorMax :type "Vector Structure"))
  (bind (_floatmin _floatmax) (`self.FloatMinMax` (.y VectorA) (.y VectorB)))
  (bind (_floatmin_2 _floatmax_2) (`self.FloatMinMax` (.z VectorA) (.z VectorB)))
  (bind (_floatmin_3 _floatmax_3) (`self.FloatMinMax` (.x VectorA) (.x VectorB)))
  (return (`KismetMathLibrary.MakeVector` _floatmin_3 _floatmin _floatmin_2) (`KismetMathLibrary.MakeVector` _floatmax_3 _floatmax _floatmax_2)))