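; Location helper library that computes obstacle-avoidance positions for characters, plus a random integer-array pick helper.
; CharacterRadar line-traces flat beams at a list of yaw angles around the actor's facing, drawing debug lines.
; ComparativeDistance turns each hit into distance and signed side ratios, which PushBackResult uses to offset backward and sideways, more strongly when closer.
; Hits overwrite rather than accumulate, so the last one determines the returned location.
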(fn `CharacterRadar`
  (params (ActorLocation :type "Vector Structure") (ActorRotation :type "Rotator Structure") (RadarStart :type "Vector Structure") (ZArray :type "Array of Float (double-precision)") (RadarLength :type "Float (double-precision)") (PushBack :type "Float (double-precision)") (IgnoreSelf :type "Actor Object Reference"))
  (returns (tCas :type "Vector Structure"))
  (locals (ActorFinalLocation :type "Vector Structure"))
  (bind _returnvalue (+ ActorLocation RadarStart))
  (set `local.ActorFinalLocation` ActorLocation)
  (for _array_element ZArray
    (bind _destination (`self.GetComparativeRotationBeam` _returnvalue ActorRotation (`KismetMathLibrary.MakeRotator` 0.0 0.0 _array_element) RadarLength))
    (bind (_outhit _returnvalue_2) (`KismetSystemLibrary.LineTraceSingleForObjects` null _returnvalue _destination (`|MakeArray` "ObjectTypeQuery3" "ObjectTypeQuery10" "ObjectTypeQuery1" "ObjectTypeQuery2" :!type "EObjectTypeQuery Enum") true (`|MakeArray` IgnoreSelf) "ForOneFrame" true (struct :`R` 1.0 :`A` 1.0) (struct :`G` 1.0 :`A` 1.0) 1.0))
    (if _returnvalue_2
      (bind (_bblockinghit _binitialoverlap _time _location _impactpoint) (`GameplayStatics.BreakHitResult` _outhit))
      (if _bblockinghit
        (bind (_distanceratio _lateralmagnitude _lateralitysign _relativelaterality) (`self.ComparativeDistance` _returnvalue _destination _impactpoint ActorRotation))
        (set `local.ActorFinalLocation` (`self.PushBackResult` _returnvalue ActorRotation PushBack _distanceratio _relativelaterality)))))
  (return (`local.ActorFinalLocation`)))

(fn `ComparativeDistance`
  (params (Start :type "Vector Structure") (End :type "Vector Structure") (HitLocation :type "Vector Structure") (RotationCenter :type "Rotator Structure"))
  (returns (DistanceRatio :type "Float (double-precision)") (LateralMagnitude :type "Float (double-precision)") (LateralitySign :type "Float (double-precision)") (RelativeLaterality :type "Float (double-precision)"))
  (bind _returnvalue (- Start HitLocation))
  (bind _returnvalue_2 (`KismetMathLibrary.Normal` (`KismetMathLibrary.GetForwardVector` RotationCenter)))
  (bind _returnvalue_3 (`KismetMathLibrary.Normal` _returnvalue))
  (bind _returnvalue_4 (`KismetMathLibrary.Dot_VectorVector` _returnvalue_2 _returnvalue_3))
  (bind _z (.z (`KismetMathLibrary.Cross_VectorVector` _returnvalue_2 _returnvalue_3)))
  (return (`KismetMathLibrary.MapRangeClamped` (`KismetMathLibrary.VSize` _returnvalue) 0.0 (`KismetMathLibrary.VSize` (- Start End)) 0.0 1.0) _returnvalue_4 (`KismetMathLibrary.SignOfFloat` _z) (* _returnvalue_4 _z)))

(fn `GetComparativeRotationBeam`
  (params (PresentLocation :type "Vector Structure") (PresentRotation :type "Rotator Structure") (AngleSeek :type "Rotator Structure") (RadarLength :type "Float (double-precision)"))
  (returns (Destination :type "Vector Structure"))
  (return (`KismetMathLibrary.MakeVector` (.x (+ PresentLocation (* (`KismetMathLibrary.GetForwardVector` (`KismetMathLibrary.ComposeRotators` PresentRotation AngleSeek)) RadarLength))) (.y (+ PresentLocation (* (`KismetMathLibrary.GetForwardVector` (`KismetMathLibrary.ComposeRotators` PresentRotation AngleSeek)) RadarLength))) (.z PresentLocation))))

(fn `GetRandomIntItem`
  (params (TargetArray :type "Array of Integer"))
  (returns (Item :type Integer))
  (bind _returnvalue (`KismetArrayLibrary.Array_Length` TargetArray))
  (bind _returnvalue_2 (`KismetMathLibrary.RandomInteger` (- _returnvalue 1)))
  (if (<= _returnvalue 0)
    (if (`KismetArrayLibrary.Array_IsValidIndex` TargetArray _returnvalue_2)
      (return (`KismetArrayLibrary.Array_Get` TargetArray _returnvalue_2))
      (else
        (return (`KismetArrayLibrary.Array_Get` TargetArray))))
    (else
      (return 0))))

(fn `PushBackResult`
  (params (PresentDestination :type "Vector Structure") (Rotation :type "Rotator Structure") (PushBack :type "Float (double-precision)") (SafeFactor :type "Float (double-precision)") (RelativeLaterality :type "Float (double-precision)"))
  (returns (Destination :type "Vector Structure"))
  (return (+ PresentDestination (* (+ (* (`KismetMathLibrary.GetForwardVector` Rotation) (* PushBack -1.0)) (* (`KismetMathLibrary.GetRightVector` Rotation) RelativeLaterality)) (- 1.0 SafeFactor)))))