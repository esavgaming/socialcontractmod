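; Blueprint function library for the tradebox mod that converts command strings to and from structs and supplies character-customization constants.
; Command parses "name|key:values;key:values" strings into a command with labeled value arrays, using "void" for missing values.
; TickerMake serializes that struct back into the same delimited format.
; BodyPartSetting and PersonalSpecs return hardcoded index groups and appearance parameter, bone and DNA option names.
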(fn `BodyPartSetting`
  (returns (Correlation :type "Array of String"))
  (return (`|MakeArray` "2,3,8" "0,1,7" "5,6,11,12")))

(fn `Command`
  (params (SourceString :type String))
  (returns (dat_CommandParams :type "/Game/ModsShared/tradeboxmod/DataStructures/dat_CommandParams Structure"))
  (locals (LabeledArray :type "Array of /Game/ModsShared/tradeboxmod/DataStructures/dat_LabeledArray Structure") (CommandReturn :type "/Game/ModsShared/tradeboxmod/DataStructures/dat_CommandParams Structure"))
  (bind _returnvalue (`KismetStringLibrary.ParseIntoArray` SourceString "|"))
  (bind _dat_commandparams (make `/Game/ModsShared/tradeboxmod/DataStructures/dat_CommandParams` (`KismetArrayLibrary.Array_Get` _returnvalue) (`local.LabeledArray`)))
  (if (> (`KismetArrayLibrary.Array_Length` _returnvalue) 1)
    (for _array_element (`KismetStringLibrary.ParseIntoArray` (`KismetArrayLibrary.Array_Get` _returnvalue 1) ";")
      (bind _returnvalue_2 (`KismetStringLibrary.ParseIntoArray` _array_element ":"))
      (if (> (`KismetArrayLibrary.Array_Length` _returnvalue_2) 1)
        (bind _item (`KismetArrayLibrary.Array_Get` _returnvalue_2))
        (`KismetArrayLibrary.Array_Add` (`local.LabeledArray`) (make `/Game/ModsShared/tradeboxmod/DataStructures/dat_LabeledArray` _item (`KismetStringLibrary.ParseIntoArray` (`KismetArrayLibrary.Array_Get` _returnvalue_2 1) ",")))
        (else
          (`KismetArrayLibrary.Array_Add` (`local.LabeledArray`) (make `/Game/ModsShared/tradeboxmod/DataStructures/dat_LabeledArray` _item (`|MakeArray` "void")))))))
  (set `local.CommandReturn` _dat_commandparams)
  (return _dat_commandparams))

(fn `PersonalSpecs`
  (returns (Scalar :type "Array of String") (Integer :type "Array of String") (Bones :type "Array of String") (DNAOptions :type "Array of String"))
  (return (`|MakeArray` "Height" "Bust" "Dick" "Eye Angle" "Eye Size" "Eye Depth" "Nose Width" "Nose Size" "Nose Curve" "Jaw Width" "Cheek Height" "Cheek Width" "Chin Width" "Ear Angle" "Ear Size" "Lip Size" "Pitch" "Physique Max" "Physique Min") (`|MakeArray` "Hair" "Facial Hair" "Face" "Eyebrow" "Eye" "Lip" "Face Warpaint" "Body Warpaint" "Hands Warpaint" "Hairline" "Facial hairline" "Skin Color" "Hair Color" "Facial Hair Color" "Eye Color" "Eyebrow Color" "Eye Makeup Color" "Lip Makeup Color" "Warpaint color" "Physique Set" "Voice Pitch") (`|MakeArray` "Full Body" "Lower Back" "Mid Back" "Upper Back" "Head" "Upper Thigh" "Mid Thigh" "Thigh" "Neck" "Upper Neck" "Hand" "Foot" "Calf" "Forearm" "Arm" "Wrist" "Clavicle" "Breast" "Penis Base" "Penis Shaft" "Penis Glande" "Jaw" "Outer Upper Lip" "Mid Outer Upper Lip" "Mid Inner Upper Lip" "Inner Upper Lip" "Outer Lower Lip" "Mid Outer Lower Lip" "Mid Inner Lower Lip" "Inner Lower Lip" "Outer Brow" "Mid Brow" "Inner Brow" "EyeScale" "Eye" "UpperEyelid" "LowerEyelid" "Nose Tip" "Nose" "Nostrills" "Philtrum" "Elbow" "Cheek Crease" "Cheek Crease Low" "Cheek Low" "Cheek Mid" "Ear" "JawSide" "Knee") (`|MakeArray` "Upper Body" "Core" "Lower Body")))

(fn `TickerMake`
  (params (CommandEntry :type "/Game/ModsShared/tradeboxmod/DataStructures/dat_CommandParams Structure"))
  (returns (ReturnValue :type String))
  (locals (FinalString :type String))
  (bind (_command _params) (break `/Game/ModsShared/tradeboxmod/DataStructures/dat_CommandParams` CommandEntry))
  (for _array_element _params
    (bind (_message _setvalues) (break `/Game/ModsShared/tradeboxmod/DataStructures/dat_LabeledArray` _array_element))
    (set `local.FinalString` (`KismetStringLibrary.Concat_StrStr` (`local.FinalString`) (`KismetStringLibrary.Concat_StrStr` _message ":" (`KismetStringLibrary.JoinStringArray` _setvalues ",")) ";")))
  (return (`KismetStringLibrary.Concat_StrStr` _command "|" (`local.FinalString`))))