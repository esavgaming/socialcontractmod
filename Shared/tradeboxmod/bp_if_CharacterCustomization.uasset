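; Blueprint interface for character customization layouts in the tradeboxmod, covering armor, uniform, makeup and tuck appearance categories.
; It declares calls to receive layout arrays, wear or store layouts by slot, apply or store them by type, and edit makeup and tuck values.
; Query functions report valid slots and slot fill, alongside toggles for mogged and pretender states.
; All functions are empty declarations, leaving behavior to implementers.
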(fn `LayoutApplyTypeArmor`
  (params (Type :type "/Game/ModsShared/tradeboxmod/DataStructures/enum_Armor Enum")))

(fn `LayoutApplyTypeMakeup`
  (params (Type :type "/Game/ModsShared/tradeboxmod/DataStructures/enum_Makeup Enum") (BaseLayout :type "CharacterLayout Structure")))

(fn `LayoutApplyTypeTuck`
  (params (Type :type "/Game/ModsShared/tradeboxmod/DataStructures/enum_Tuck Enum") (BaseLayouy :type "CharacterLayout Structure")))

(fn `LayoutEditMakeup`
  (params (Index :type Integer) (Back :type Boolean)))

(fn `LayoutEditTuck`
  (params (Value :type "Float (double-precision)") (Index :type Integer)))

(fn `LayoutForceChange`
  (params (BaseLayout :type "CharacterLayout Structure")))

(fn `LayoutGetArmorSlotFill`
  (params (Original :type "CharacterLayout Structure") (Slot :type Integer))
  (returns (Sample :type "CharacterLayout Structure"))
  (return))

(fn `LayoutGetArmorValidSlots`
  (returns (ValidSlots :type String))
  (return ""))

(fn `LayoutGetMakeupSlotFill`
  (params (Original :type "CharacterLayout Structure") (Slot :type Integer))
  (returns (Sample :type "CharacterLayout Structure"))
  (return))

(fn `LayoutGetMakeupValidSlots`
  (returns (ValidSlots :type String))
  (return ""))

(fn `LayoutGetTuckSlotFill`
  (params (Original :type "CharacterLayout Structure") (Slot :type Integer))
  (returns (Sample :type "CharacterLayout Structure"))
  (return))

(fn `LayoutGetTuckValidSlots`
  (returns (ValidSlots :type String))
  (return ""))

(fn `LayoutGetTypeArmorFill`
  (params (TypeGet :type "/Game/ModsShared/tradeboxmod/DataStructures/enum_Armor Enum"))
  (returns (Sample :type "CharacterLayout Structure"))
  (return))

(fn `LayoutMakeupReverseFill`)

(fn `LayoutOriginateCurrent`
  (params (Reverse :type Boolean)))

(fn `LayoutPretender`
  (params (Pretend :type Boolean)))

(fn `LayoutReceiveArmorArray`
  (params (BaseLayout :type "CharacterLayout Structure")))

(fn `LayoutReceiveMakeUpArray`
  (params (BaseLayout :type "CharacterLayout Structure")))

(fn `LayoutReceiveTuckArray`
  (params (BaseLayout :type "CharacterLayout Structure")))

(fn `LayoutReceiveUniformArray`
  (params (BaseLayout :type "CharacterLayout Structure")))

(fn `LayoutSetMogged`
  (params (bIsMogged :type Boolean)))

(fn `LayoutStoreSlotArmor`
  (params (Slot :type Integer) (BaseLayout :type "CharacterLayout Structure")))

(fn `LayoutStoreSlotMakeup`
  (params (Slot :type Integer) (BaseLayout :type "CharacterLayout Structure")))

(fn `LayoutStoreSlotTuck`
  (params (Slot :type Integer) (BaseLayout :type "CharacterLayout Structure")))

(fn `LayoutStoreTypeArmor`
  (params (Type :type "/Game/ModsShared/tradeboxmod/DataStructures/enum_Armor Enum") (BaseLayout :type "CharacterLayout Structure")))

(fn `LayoutTuckReverseFill`)

(fn `LayoutWearSlotArmor`
  (params (Slot :type Integer)))

(fn `LayoutWearSlotMakeup`
  (params (Slot :type Integer)))

(fn `LayoutWearSlotTuck`
  (params (Slot :type Integer)))